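; BP_ActionComponent is a lightweight, GAS-style action component that owns and runs gameplay action objects for its owning actor.
; On BeginPlay it instantiates each configured action class, and OneTimeAction can add and optionally auto-start more at runtime.
; Actions start by matching their label tag, gated by CanStart against an active gameplay tag container, and stop on an exact tag match.
; Events add or remove active tags and actions.
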(event Custom|StartActionByTag
  (params (Tag :type Gameplay%20Tag%20Structure) (IsAI :type Boolean))
  ;[0.15 0.15 0.15 0.5] StartActionByTag
  (for _array_element (Variables|Default|GetSActionObject)
    (if (and (Default|CanStart _array_element (Variables|Default|GetActiveGamePlayTagContainer) self) (GameplayTags|MatchesTag (Variables|/Game/ActionComponent/SActionClass.SActionClass_C|GetLebel%20Tag _array_element) Tag))
      (Default|StartAction _array_element (Utilities|Struct|MakeStruct_GAS_System self (Components|GetOwner) Tag IsAI)))))

(event Custom|StopActionTag
  (params (Tag :type Gameplay%20Tag%20Structure) (IsAI :type Boolean))
  ;[0.15 0.15 0.15 0.5] StopAction By Tag
  (for _array_element (Variables|Default|GetSActionObject)
    (if (== (Variables|/Game/ActionComponent/SActionClass.SActionClass_C|GetLebel%20Tag _array_element) Tag)
      (Default|StopAction _array_element (Utilities|Struct|MakeStruct_GAS_System self (Components|GetOwner) Tag IsAI)))))

(event Custom|Add%20Action
  ;[0.15 0.15 0.15 0.5] Loop Action To Start
  (for _array_element (Variables|Default|GetSAction)
    (bind _returnvalue (Game|ConstructObjectfromClass self _array_element))
    (Utilities|Array|Add (Variables|Default|GetSActionObject) _returnvalue)))

(event Custom|OneTimeAction
  (params (SAction :type S%20Action%20Class%20Class%20Reference) (StartFunctionByTag :type Gameplay%20Tag%20Structure))
  (bind _self self)
  ;[0.15 0.15 0.15 0.5] One Time Start
  (bind _returnvalue (Game|ConstructObjectfromClass _self SAction))
  (if (Default|CanStart _returnvalue (Variables|Default|GetActiveGamePlayTagContainer) _self)
    (Utilities|Array|Add (Variables|Default|GetSActionObject) _returnvalue)
    (if (Variables|/Game/ActionComponent/SActionClass.SActionClass_C|GetbDoesAutoStart _returnvalue)
      (Default|StartAction _returnvalue (Utilities|Struct|MakeStruct_GAS_System self (Components|GetOwner) StartFunctionByTag)))))

(event Custom|RemoveAction
  (params (Action :type S%20Action%20Class%20Object%20Reference))
  (Utilities|Array|RemoveItem (Variables|Default|GetSActionObject) Action))

(event EventBeginPlay
  (CallFunction|AddAction)
  (Utilities|FlowControl|DelayUntilNextTick))

(event EventAddTag
  (params (AddTag :type Gameplay%20Tag%20Structure))
  (GameplayTags|AddGameplayTag (Variables|Default|GetActiveGamePlayTagContainer) AddTag :!class /Script/GameplayTags.BlueprintGameplayTagLibrary))

(event EventRemoveTag
  (params (RemoveTag :type Gameplay%20Tag%20Structure))
  (GameplayTags|RemoveGameplayTag (Variables|Default|GetActiveGamePlayTagContainer) RemoveTag :!class /Script/GameplayTags.BlueprintGameplayTagLibrary))

(fn GetActiveGamePlayTagContainer
  (return (Variables|Default|GetActiveGamePlayTagContainer)))