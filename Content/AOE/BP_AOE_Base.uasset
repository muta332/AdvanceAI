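; Base area-of-effect actor that finds actors within a radius and broadcasts each one through an OnAOEOverlapActor dispatcher.
; Trigger runs a sphere overlap at the actor's location, optionally drawn for debugging, and can fire automatically shortly after BeginPlay.
; IgnoreInstigator excludes the Owner rather than the Instigator.
; Each hit prints its name and sets a short lifespan on the AOE, so an empty overlap leaves the actor alive.
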(event Custom|Trigger
  (CallFunction|SpawnAOESphere))

(event Custom|SpawnAOESphere
  (if (Variables|Default|GetDrawDebugSphere)
    (Rendering|Debug|DrawDebugSphere (Transformation|GetActorLocation) (Variables|Default|GetRadius) 12 "(R=1.000000,G=0.000000,B=0.802695,A=1.000000)" 1.0 1.0))
  (bind (_outactors _returnvalue) (Collision|SphereOverlapActors (Transformation|GetActorLocation) (Variables|Default|GetRadius) (Utilities|Array|MakeArray "ObjectTypeQuery3" "ObjectTypeQuery7") 0 (Utilities|Array|MakeArray (select (Variables|Default|GetIgnoreInstigator) (Components|GetOwner) 0))))
  (if _returnvalue
    (for _array_element _outactors
      (Default|CallOnAOEOverlapActor _array_element)
      (Development|PrintString (Utilities|GetDisplayName _array_element) true true "(R=0.000000,G=0.660000,B=1.000000,A=1.000000)" 2.0 "1")
      (Actor|SetLifeSpan 1.0))))

(event EventBeginPlay
  (if (Variables|Default|GetTriggerOnBeginPlay)
    (Utilities|FlowControl|Delay 0.1)
    (CallFunction|Trigger)))

(fn ConstructionScript)