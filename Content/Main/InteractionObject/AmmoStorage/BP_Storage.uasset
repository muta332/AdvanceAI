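; Interactable ammo storage that refills the reserve ammo of the interacting character's weapon from a limited pool, initialized to MaxAmmo at construction.
; Interact passes the used storage amount to the weapon's gun system, then re-reads it to decrement the clamped pool, or prints "Storage Full".
; GetInteractText supplies the prompt and remaining count.
; The player widget refresh also requires IsAI, which is set only when the BP_Player cast fails.
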(event EventBeginPlay)

(event Collision|EventActorBeginOverlap
  (params (OtherActor :type Actor%20Object%20Reference)))

(event EventTick
  (params (DeltaSeconds :type Float%20%28single-precision%29)))

(event EventInteract
  (params (Instigator :type Actor%20Object%20Reference))
  (|CallParentFunction Instigator)
  (if (CallFunction|CheckRemainingAmmo)
    (bind _returnvalue (Class|GCharacterInterface|GetCharacter(Message) Instigator))
    (bind _asbp_player (Utilities|Casting|CastToBP_Player _returnvalue)
      (:then
        _)
      (:CastFailed
        (Variables|Default|SetIsAI true)))
    (if (!= (Variables|/Script/AdvanceAI.GGunSystem|GetCurrentStorage (Actor|GetComponentbyClass (Variables|/Game/Main/Player/BP_Player.BP_Player_C|GetWeapon _returnvalue) "/Script/AdvanceAI.GGunSystem")) (Variables|/Script/AdvanceAI.GGunSystem|GetMaxAmmoStorage (Actor|GetComponentbyClass (Variables|/Game/Main/Player/BP_Player.BP_Player_C|GetWeapon _returnvalue) "/Script/AdvanceAI.GGunSystem")))
      (Class|GGunSystem|SetAmmoStorage (Actor|GetComponentbyClass (Variables|/Game/Main/Player/BP_Player.BP_Player_C|GetWeapon _returnvalue) "/Script/AdvanceAI.GGunSystem") (Class|GGunSystem|GetUsedAmmoAmountinStorage (Actor|GetComponentbyClass (Variables|/Game/Main/Player/BP_Player.BP_Player_C|GetWeapon _returnvalue) "/Script/AdvanceAI.GGunSystem")))
      (Variables|Default|SetRemainig%20Ammo%20 (Math|Integer|Clamp(Integer) (- (Variables|Default|GetRemainig%20Ammo%20) (Class|GGunSystem|GetUsedAmmoAmountinStorage (Actor|GetComponentbyClass (Variables|/Game/Main/Player/BP_Player.BP_Player_C|GetWeapon _returnvalue) "/Script/AdvanceAI.GGunSystem"))) 0 (Variables|Default|GetMax%20Ammo)))
      (if (and (Utilities|IsValid _asbp_player) (Variables|Default|GetIsAI))
        (bind _interactionwidget (Variables|/Game/Main/Player/BP_Player.BP_Player_C|GetInteractionWidget _asbp_player)
          (:then
            (Class|GInteractionWidget|SetRemainingAmmoText _interactionwidget (Utilities|Text|ToText(String) (Utilities|String|Append "Remaining Ammo" "         " (Utilities|String|ToString(Integer) (Variables|Default|GetRemainig%20Ammo%20))))))
          (:else)))
      (else
        (Development|PrintString "Storage Full" true true "(R=1.000000,G=0.000000,B=0.063568,A=1.000000)" 2.0 "Storage")))))

(fn ConstructionScript
  (Variables|Default|SetRemainig%20Ammo%20 (Variables|Default|GetMax%20Ammo)))

(fn GetInteractText
  (return (Variables|Default|GetWidgetInteractionText) (Utilities|Text|ToText(String) (Utilities|String|Append "Remaining Ammo" "         " (Utilities|String|ToString(Integer) (Variables|Default|GetRemainig%20Ammo%20))))))

(fn CheckRemainingAmmo
  (return (not (<= (Variables|Default|GetRemainig%20Ammo%20) 0))))