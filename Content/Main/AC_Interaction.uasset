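; Player interaction component that detects actors tagged "Interaction Actor" in front of the BP_Player follow camera.
; Tick runs a short forward sphere trace only when the camera moves or the dot product of normalized trace end points drops below a threshold.
; A tagged hit is stored and triggers CallWidgetInteract, while losing any hit clears it through CallNoInteractActor.
; Interact sends InteractMessage to the stored actor with the owner.
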(event Custom|Interact%20Actor
  (bind _output_get (Variables|Default|SetTraceHitActor (.HitActor (Collision|BreakHitResult (stale EventTick _outhit)))))
  (Default|CallWidgetInteract _output_get)
  (Variables|Default|SetInteracting true))

(event Custom|Not%20Interacting
  (if (Variables|Default|GetInteracting)
    (Default|CallNoInteractActor)
    (Variables|Default|SetInteracting false)
    (Variables|Default|SetTraceHitActor 0)))

(event Custom|Interact
  (Class|BPIInteraction|Interact(Message) (Variables|Default|GetTraceHitActor) (Components|GetOwner)))

(event EventBeginPlay
  (bind _asbp_player (Utilities|Casting|CastToBP_Player (Components|GetOwner)))
  (bind _output_get (Variables|Default|SetPlayer _asbp_player))
  (Variables|Default|SetCamera (Variables|/Script/AdvanceAI.BasePlayerCharacter|GetFollowCamera _output_get)))

(event EventTick
  (params (DeltaSeconds :type Float%20%28single-precision%29))
  (bind (_start _end) (CallFunction|CamearPos))
  (if (or (< (CallFunction|GetCameraRotationDegree _end) 0.98) (Utilities|Operators|NotEqual(!=) _start (Variables|Default|GetLast%20Camera%20Location) 0.0001))
    (bind (_outhit _returnvalue) (Collision|SphereTraceForObjects _start _end 1e+02 (Utilities|Array|MakeArray "ObjectTypeQuery3" "ObjectTypeQuery2") false 0 "None" true "(R=1.000000,G=0.000000,B=0.000000,A=1.000000)" "(R=0.000000,G=1.000000,B=0.000000,A=1.000000)" 0.5))
    (Variables|Default|SetSetLastRotation _end)
    (Variables|Default|SetLast%20Camera%20Location _start)
    (Utilities|IsValid (.HitActor (Collision|BreakHitResult _outhit))
      (:Is%20Valid
        (if (Math|Boolean|ANDBoolean _returnvalue (Actor|ActorHasTag (.HitActor (Collision|BreakHitResult _outhit)) "Interaction Actor") (not (Variables|Default|GetInteracting)))
          (CallFunction|InteractActor)))
      (:Is%20Not%20Valid
        (CallFunction|NotInteracting)))))

(fn CamearPos
  (bind _camera (Variables|Default|GetCamera))
  (bind _returnvalue (Transformation|GetWorldLocation _camera))
  (return _returnvalue (+ _returnvalue (* (Math|Vector|GetForwardVector (Transformation|GetWorldRotation _camera)) 5e+02))))

(fn GetCameraRotationDegree
  (params (Current%20Rotation :type Vector))
  (return (Math|Vector|DotProduct (Math|Vector|Normalize (Variables|Default|GetSetLastRotation)) (Math|Vector|Normalize Current%20Rotation))))