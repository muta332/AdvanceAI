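; Third-person shooter player character that spawns an attached rifle and handles stances, zoom, firing, interaction and grenade throws.
; Input delegates to the GunSystem, interaction and action components, whose ammo and interaction events update widgets.
; A gameplay tag container tracks stance, zoom and montage guarding; stances set walk speed, and firing halts movement until it ends.
; It also supplies left-hand IK and grenade spawn transforms, plus debug keys for camera offset and slow motion.
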(event Custom|StanceChangeSprint
  ;[0.15 0.1168 0 0.5] StanceChange
  (if (not (GameplayTags|HasTag (Variables|Default|GetActiveGamePlayTagContainer) "(TagName=\"Stance.Crouching\")"))
    (CallFunction|OnStanceChange "(TagName=\"Stance.Sprinting\")")))

(event Custom|StanceChangeRunning
  ;[0.15 0.1168 0 0.5] StanceChange
  (if (not (GameplayTags|HasTag (Variables|Default|GetActiveGamePlayTagContainer) "(TagName=\"Stance.Crouching\")"))
    (CallFunction|OnStanceChange "(TagName=\"Stance.Running\")")))

(event Custom|MontageInterrupted
  ;[0.15 0.15 0.15 0.5] Montage Funtion
  ;;[0.15 0.01724 0 0.5] MontageEnd or Interrupt
  (GameplayTags|RemoveGameplayTag (Variables|Default|GetActiveGamePlayTagContainer) "(TagName=\"Status.Shooting\")" :!class /Script/GameplayTags.BlueprintGameplayTagLibrary)
  (GameplayTags|RemoveGameplayTag (Variables|Default|GetActiveGamePlayTagContainer) "(TagName=\"AnimGaurd.AnimPlaying\")" :!class /Script/GameplayTags.BlueprintGameplayTagLibrary))

(event Custom|OnFireEnded_Event
  (bind _activegameplaytagcontainer (Variables|Default|GetActiveGamePlayTagContainer))
  ;[0.15 0.15 0.15 0.5] On Fire Start and End
  (Pawn|Components|CharacterMovement|SetMovementMode (Variables|Character|GetCharacterMovement) "MOVE_Walking" 0)
  (GameplayTags|RemoveGameplayTag _activegameplaytagcontainer "(TagName=\"Status.Shooting\")" :!class /Script/GameplayTags.BlueprintGameplayTagLibrary)
  (if (not (GameplayTags|HasTag _activegameplaytagcontainer "(TagName=\"Stance.Crouching\")"))
    (CallFunction|SetSpeed (Variables|Default|GetMax%20Run%20speed))
    (else
      (CallFunction|SetSpeed (Variables|Default|GetMax%20Crouch/Walk%20Speed)))))

(event Custom|GunTrigger
  ;[0.15 0.15 0.15 0.5] GunTrigger
  (Default|Triggered (Variables|Default|GetGunSystemComponent)))

(event Custom|IA_ZoomingStarted
  ;[0.15 0.15 0.15 0.5] Execute when Zoom starts
  (GameplayTags|AddGameplayTag (Variables|Default|GetActiveGamePlayTagContainer) "(TagName=\"Camera.ZoomIn\")" :!class /Script/GameplayTags.BlueprintGameplayTagLibrary)
  (bind _length (Timeline|CameraTimeLine Play)
    (:Update
      (Variables|/Script/Engine.SpringArmComponent|SetSocketOffset (Variables|Default|GetCameraBoom) (Math|Vector|Lerp(Vector) (Variables|Default|GetRunCameraOffset) (Utilities|Select :Index (Variables|Default|GetStance) :NewEnumerator0 (Variables|Default|GetCrouchCameraZoomLocation) :NewEnumerator1 (Variables|Default|GetNormalCamereaOffset) :NewEnumerator2 "0, 0, 0" :NewEnumerator3 "0, 0, 0") _length)))
    (:Finished
      (if (GameplayTags|HasTag (Variables|Default|GetActiveGamePlayTagContainer) "(TagName=\"Camera.ZoomIn\")")
        (Widget|SetVisibility (Variables|/Game/Main/PlayerWidget/WBP_Main.WBP_Main_C|GetWBP_Crosshair (Variables|Default|GetPlayerHud)) "Visible")))))

(event Custom|GunTriggerEnd
  ;[0.15 0.15 0.15 0.5] GunTrigger
  (Default|TriggerReleased (Variables|Default|GetGunSystemComponent)))

(event Custom|CameraBoomOffset
  ;[0.15 0.15 0.15 0.5] CameraBoomOffset
  (if (not (GameplayTags|HasTag (Variables|Default|GetActiveGamePlayTagContainer) "(TagName=\"Camera.ZoomIn\")"))
    _))

(event Custom|Reloading
  ;[0.15 0.15 0.15 0.5] GunTrigger
  (Default|Reloading (Variables|Default|GetGunSystemComponent)))

(event Custom|OnFireStarted_Event
  ;[0.15 0.15 0.15 0.5] On Fire Start and End
  (CallFunction|SetSpeed 0.0)
  (Pawn|Components|CharacterMovement|SetMovementMode (Variables|Character|GetCharacterMovement) "MOVE_None" 0))

(event Custom|HideWeapon
  (params (bHideWeapon :type Boolean))
  ;[0.15 0.15 0.15 0.5] ThrowGranade
  (Development|SetHiddeninGame (Variables|/Game/Main/Wepon/Gun/Base_Gun.Base_Gun_C|GetGunSkeletalMesh (Variables|Default|GetWeapon)) bHideWeapon false))

(event Custom|On%20Reload%20Finished_Event
  (params (Ammo :type Integer) (Storage%20Ammo :type Integer))
  (bind _playerhud (Variables|Default|GetPlayerHud))
  ;[0.15 0.15 0.15 0.5] Reloading
  (Default|SetStorageAmmo _playerhud (Utilities|Text|ToText(Integer) Storage%20Ammo))
  (Default|SetRemainingAmmo _playerhud (Utilities|Text|ToText(Integer) Ammo)))

(event Custom|StanceChangeWalking
  ;[0.15 0.1168 0 0.5] StanceChange
  (Utilities|FlowControl|FlipFlop
    (:A
      (CallFunction|OnStanceChange "(TagName=\"Stance.Walking\")"))
    (:B
      (CallFunction|OnStanceChange "(TagName=\"Stance.Running\")"))))

(event Custom|On%20Update%20Ammo_Event
  (params (Ammo :type Integer))
  ;[0.15 0.15 0.15 0.5] Reloading
  (Default|SetRemainingAmmo (Variables|Default|GetPlayerHud) (Utilities|Text|ToText(Integer) Ammo)))

(event Custom|WidgetInteract
  (params (InteractActor :type Actor%20Object%20Reference))
  (bind (_text _remainingammo) (Class|BPIInteraction|GetInteractText(Message) InteractActor))
  (bind _returnvalue (UserInterface|CreateWidget "/Game/Main/Wepon/InteractionObject/InteractionWidget/WBP_InteractionWidget.WBP_InteractionWidget_C" (Game|GetPlayerController 0) _text InteractActor _remainingammo))
  (UserInterface|Viewport|AddtoViewport _returnvalue 0))

(event Custom|UpdateStorage
  (params (CurrentStorage :type Integer))
  ;[0.15 0.15 0.15 0.5] Reloading
  (Default|SetStorageAmmo (Variables|Default|GetPlayerHud) (Utilities|Text|ToText(Integer) CurrentStorage)))

(event Custom|Switch%20GunMode
  (Default|SwtichFiringMode (Variables|Default|GetGunSystemComponent)))

(event Custom|Spawn%20Primary%20Weapon
  (bind _self self)
  ;[0.15 0.15 0.15 0.5] Weapon
  (bind _returnvalue (Game|SpawnActorfromClass "/Game/Main/Wepon/Gun/AR/BP_ARRifle.BP_ARRifle_C" (Math|Transform|MakeTransform "0, 0, 0" "0, 0, 0" "1.000000,1.000000,1.000000") "Undefined" "MultiplyWithRoot" _self _self))
  (bind _output_get (Variables|Default|SetWeapon _returnvalue))
  (Variables|Default|SetGunSystemComponent (Actor|GetComponentbyClass _output_get "/Game/Main/GunSystem/GunSystem.GunSystem_C"))
  (Transformation|AttachComponentToComponent (Variables|Default|GetWeapon) (Variables|Character|GetMesh) (Variables|Default|GetAttachWeaponToSocket) "SnapToTarget" "SnapToTarget" "SnapToTarget" true))

(event Custom|CreateWidget
  (bind _gunsystemcomponent (Variables|Default|GetGunSystemComponent))
  ;[0.15 0.15 0.15 0.5] Widget
  (bind _returnvalue (UserInterface|CreateWidget "/Game/Main/PlayerWidget/WBP_Main.WBP_Main_C" (Game|GetPlayerController 0) (Variables|/Game/Main/GunSystem/GunSystem.GunSystem_C|GetCurrentStorage _gunsystemcomponent) (Variables|/Game/Main/GunSystem/GunSystem.GunSystem_C|GetAmmo%20In%20Mag _gunsystemcomponent)))
  (bind _output_get (Variables|Default|SetPlayerHud _returnvalue))
  (UserInterface|Viewport|AddtoViewport _output_get 0))

(event Custom|NoInteraction
  (Widget|RemovefromParent (stale Custom|WidgetInteract _returnvalue)))

(event Custom|Funtion%20Binding
  (bind _gunsystemcomponent (Variables|Default|GetGunSystemComponent))
  ;[0.15 0.15 0.15 0.5] Bind Events
  (EventDispatchers|AssignOnMontageEnded (Variables|Default|GetAnimInstance) (EventDispatchers|CreateEvent :!event Custom|OnMontageEnded_Event))
  (EventDispatchers|AssignOnFireEnded _gunsystemcomponent (EventDispatchers|CreateEvent :!event Custom|OnFireEnded_Event))
  (EventDispatchers|AssignOnFireStarted _gunsystemcomponent (EventDispatchers|CreateEvent :!event Custom|OnFireStarted_Event))
  (EventDispatchers|AssignOnReloadFinished _gunsystemcomponent (EventDispatchers|CreateEvent :!event Custom|On%20Reload%20Finished_Event))
  (EventDispatchers|AssignOnUpdateMag _gunsystemcomponent (EventDispatchers|CreateEvent :!event Custom|On%20Update%20Ammo_Event))
  (EventDispatchers|BindEventtoWidgetInteract (Variables|Default|GetAC_Interaction) (EventDispatchers|CreateEvent :!event Custom|WidgetInteract))
  (EventDispatchers|BindEventtoNoInteractActor (Variables|Default|GetAC_Interaction) (EventDispatchers|CreateEvent :!event Custom|NoInteraction))
  (EventDispatchers|BindEventtoUpdateCurrentStorage (Variables|/Game/Main/Wepon/Gun/Base_Gun.Base_Gun_C|GetGunSystem (Variables|Default|GetWeapon)) (EventDispatchers|CreateEvent :!event Custom|UpdateStorage)))

(event Custom|OnMontageEnded_Event
  (params (Montage :type Anim%20Montage%20Object%20Reference) (bInterrupted :type Boolean))
  ;[0.15 0.15 0.15 0.5] Montage Funtion
  ;;[0.15 0.01724 0 0.5] MontageEnd or Interrupt
  (if (not bInterrupted)
    (CallFunction|MontageEnd)
    (else
      (CallFunction|MontageInterrupted))))

(event Custom|StanceCrouching
  ;[0.15 0.1168 0 0.5] StanceChange
  (Utilities|FlowControl|FlipFlop
    (:A
      (CallFunction|OnStanceChange "(TagName=\"Stance.Crouching\")")
      (Variables|Default|SetStance "NewEnumerator0")
      (CallFunction|IAZoomingStarted))
    (:B
      (CallFunction|OnStanceChange "(TagName=\"Stance.Running\")")
      (Variables|Default|SetStance "NewEnumerator1")
      (CallFunction|IAZoomingStarted))))

(event Custom|Set%20Actor%20Rotation%20to%20Control%20Rotation
  (params (isShooting :type Boolean))
  (bind _returnvalue (Pawn|GetController))
  (bind _returnvalue_2 (Transformation|GetActorForwardVector))
  (bind _returnvalue_3 (Transformation|GetActorForwardVector _returnvalue))
  (bind _returnvalue_4 (* _returnvalue_3 5e+03))
  (bind _returnvalue_5 (Math|Rotator|FindLookatRotation _returnvalue_2 _returnvalue_4))
  ;[0.15 0.15 0.15 0.5] Set Actor Rotation
  (if isShooting
    (Transformation|SetActorRotation (Math|Rotator|MakeRotator 0.0 0.0 (.yaw _returnvalue_5)))
    (else
      (Transformation|SetActorRotation (Math|Rotator|MakeRotator 0.0 0.0 (.yaw _returnvalue_5))))))

(event Custom|On%20Stance%20Change
  (params (Stance%20Tag :type Gameplay%20Tag%20Structure))
  (bind _activegameplaytagcontainer (Variables|Default|GetActiveGamePlayTagContainer))
  ;[0.15 0.15 0.15 0.5] Stance Change
  (CallFunction|TagBatchDelete "(TagName=\"Stance\")")
  (|SwitchGameplayTag Stance%20Tag
    (:Stance.Crouching
      (GameplayTags|AddGameplayTag _activegameplaytagcontainer "(TagName=\"Stance.Crouching\")" :!class /Script/GameplayTags.BlueprintGameplayTagLibrary)
      (CallFunction|SetSpeed (Variables|Default|GetMax%20Crouch/Walk%20Speed)))
    (:Stance.Running
      (GameplayTags|AddGameplayTag _activegameplaytagcontainer "(TagName=\"Stance.Running\")" :!class /Script/GameplayTags.BlueprintGameplayTagLibrary)
      (CallFunction|SetSpeed (Variables|Default|GetMax%20Run%20speed)))
    (:Stance.Sprinting
      (GameplayTags|AddGameplayTag _activegameplaytagcontainer "(TagName=\"Stance.Sprinting\")" :!class /Script/GameplayTags.BlueprintGameplayTagLibrary)
      (CallFunction|SetSpeed (Variables|Default|GetMax%20Sprint%20Speed)))
    (:Stance.Walking
      (GameplayTags|AddGameplayTag _activegameplaytagcontainer "(TagName=\"Stance.Walking\")" :!class /Script/GameplayTags.BlueprintGameplayTagLibrary)
      (CallFunction|SetSpeed (Variables|Default|GetMax%20Crouch/Walk%20Speed)))))

(event Custom|MontageEnd
  (bind _activegameplaytagcontainer (Variables|Default|GetActiveGamePlayTagContainer))
  ;[0.15 0.15 0.15 0.5] Montage Funtion
  ;;[0.15 0.01724 0 0.5] MontageEnd or Interrupt
  (GameplayTags|RemoveGameplayTag _activegameplaytagcontainer "(TagName=\"Status.Shooting\")" :!class /Script/GameplayTags.BlueprintGameplayTagLibrary)
  (GameplayTags|RemoveGameplayTag _activegameplaytagcontainer "(TagName=\"AnimGaurd.AnimPlaying\")" :!class /Script/GameplayTags.BlueprintGameplayTagLibrary))

(event Input|EnhancedActionEvents|EnhancedInputActionIA_Attack
  (params (ActionValue :type Boolean) (ElapsedSeconds :type Float%20%28double-precision%29) (TriggeredSeconds :type Float%20%28double-precision%29) (InputAction :type Input%20Action%20Object%20Reference :default "/Game/ThirdPerson/Input/Actions/IA_Attack.IA_Attack"))
  ;[0.15 0.15 0.15 0.5] InputAction
  (:Triggered
    (CallFunction|SetActorRotationtoControlRotation false))
  (:Started
    (CallFunction|GunTrigger))
  (:Completed
    (CallFunction|GunTriggerEnd)))

(event Input|EnhancedActionEvents|EnhancedInputActionIA_ThrowGranade
  (params (ActionValue :type Boolean) (ElapsedSeconds :type Float%20%28double-precision%29) (TriggeredSeconds :type Float%20%28double-precision%29) (InputAction :type Input%20Action%20Object%20Reference :default "/Game/ThirdPerson/Input/Actions/IA_ThrowGranade.IA_ThrowGranade"))
  ;[0.15 0.15 0.15 0.5] InputAction
  (:Started
    (Default|OneTimeAction (Variables|Default|GetBP_ActionComponent) "/Game/ActionComponent/GranadeAction.GranadeAction_C" "(TagName=\"GranadeSystem\")")))

(event Input|EnhancedActionEvents|EnhancedInputActionIA_ZoomIn
  (params (ActionValue :type Boolean) (ElapsedSeconds :type Float%20%28double-precision%29) (TriggeredSeconds :type Float%20%28double-precision%29) (InputAction :type Input%20Action%20Object%20Reference :default "/Game/ThirdPerson/Input/Actions/IA_ZoomIn.IA_ZoomIn"))
  ;[0.15 0.15 0.15 0.5] CameraTimeLine Not used
  (:Triggered
    (CallFunction|SetActorRotationtoControlRotation false))
  (:Started
    (CallFunction|IAZoomingStarted))
  (:Completed
    (Widget|SetVisibility (Variables|/Game/Main/PlayerWidget/WBP_Main.WBP_Main_C|GetWBP_Crosshair (Variables|Default|GetPlayerHud)) "Visible")
    (GameplayTags|RemoveGameplayTag (Variables|Default|GetActiveGamePlayTagContainer) "(TagName=\"Camera.ZoomIn\")" :!class /Script/GameplayTags.BlueprintGameplayTagLibrary)))

(event Input|EnhancedActionEvents|EnhancedInputActionIA_Sprint
  (params (ActionValue :type Boolean) (ElapsedSeconds :type Float%20%28double-precision%29) (TriggeredSeconds :type Float%20%28double-precision%29) (InputAction :type Input%20Action%20Object%20Reference :default "/Game/ThirdPerson/Input/Actions/IA_Sprint.IA_Sprint"))
  ;[0.15 0.15 0.15 0.5] InputAction
  (:Started
    (CallFunction|StanceChangeSprint))
  (:Completed
    (CallFunction|StanceChangeRunning)))

(event Input|EnhancedActionEvents|EnhancedInputActionIA_Walk
  (params (ActionValue :type Boolean) (ElapsedSeconds :type Float%20%28double-precision%29) (TriggeredSeconds :type Float%20%28double-precision%29) (InputAction :type Input%20Action%20Object%20Reference :default "/Game/ThirdPerson/Input/Actions/IA_Walk.IA_Walk"))
  ;[0.15 0.15 0.15 0.5] InputAction
  (:Started
    (CallFunction|StanceChangeWalking)))

(event Input|EnhancedActionEvents|EnhancedInputActionIA_Crouch
  (params (ActionValue :type Boolean) (ElapsedSeconds :type Float%20%28double-precision%29) (TriggeredSeconds :type Float%20%28double-precision%29) (InputAction :type Input%20Action%20Object%20Reference :default "/Game/ThirdPerson/Input/Actions/IA_Crouch.IA_Crouch"))
  ;[0.15 0.15 0.15 0.5] InputAction
  (:Started
    (CallFunction|StanceCrouching)))

(event Input|EnhancedActionEvents|EnhancedInputActionIA_ChangeCameraBoomOffset
  (params (ActionValue :type Boolean) (ElapsedSeconds :type Float%20%28double-precision%29) (TriggeredSeconds :type Float%20%28double-precision%29) (InputAction :type Input%20Action%20Object%20Reference :default "/Game/ThirdPerson/Input/Actions/IA_ChangeCameraBoomOffset.IA_ChangeCameraBoomOffset"))
  ;[0.15 0.15 0.15 0.5] InputAction
)

(event Input|EnhancedActionEvents|EnhancedInputActionIA_FiringMode
  (params (ActionValue :type Boolean) (ElapsedSeconds :type Float%20%28double-precision%29) (TriggeredSeconds :type Float%20%28double-precision%29) (InputAction :type Input%20Action%20Object%20Reference :default "/Game/ThirdPerson/Input/Actions/IA_FiringMode.IA_FiringMode"))
  (:Started
    (CallFunction|SwitchGunMode)))

(event Input|EnhancedActionEvents|EnhancedInputActionIA_Reload
  (params (ActionValue :type Boolean) (ElapsedSeconds :type Float%20%28double-precision%29) (TriggeredSeconds :type Float%20%28double-precision%29) (InputAction :type Input%20Action%20Object%20Reference :default "/Game/ThirdPerson/Input/Actions/IA_Reload.IA_Reload"))
  ;[0.15 0.15 0.15 0.5] InputAction
  (:Started
    (CallFunction|Reloading)))

(event Input|EnhancedActionEvents|EnhancedInputActionIA_Interaction
  (params (ActionValue :type Boolean) (ElapsedSeconds :type Float%20%28double-precision%29) (TriggeredSeconds :type Float%20%28double-precision%29) (InputAction :type Input%20Action%20Object%20Reference :default "/Game/ThirdPerson/Input/Actions/IA_Interaction.IA_Interaction"))
  ;[0.15 0.15 0.15 0.5] InputAction
  (:Started
    (Default|Interact (Variables|Default|GetAC_Interaction))))

(event EventBeginPlay
  ;[0.15 0.15 0.15 0.5] Event BeginPlay
  (CallFunction|SpawnPrimaryWeapon)
  (Variables|Default|SetAnimInstance (Components|SkeletalMesh|GetAnimInstance (Variables|Character|GetMesh)))
  (CallFunction|CreateWidget)
  (CallFunction|FuntionBinding)
  (bind _asabp_character_rifle (Utilities|Casting|CastToABP_CharacterRifle (Variables|Default|GetAnimInstance)))
  (Variables|Default|SetAs%20ABP%20Character%20Rifle _asabp_character_rifle))

(event EventPlayMovementAnimation
  (params (StartMontage :type Boolean) (ForwardDirection :type Integer) (RightDirection :type Integer))
  ;[0.15 0.15 0.15 0.5] Play Dynamic Movement Animation
)

(event EventTick
  (params (DeltaSeconds :type Float%20%28single-precision%29)))

(event EventPlayAnimation
  (params (AnimMontageStuct :type Struct%20Montage%20Structure))
  (bind (_montagetoplay _inplayrate _sectionname _stopallmontages) (Utilities|Struct|BreakStruct_Montage AnimMontageStuct))
  ;[0.15 0.15 0.15 0.5] Montage Funtion
  ;;[0 0.15 0.1298 0.5] Montage Begin
  (if (not (GameplayTags|HasTag (Variables|Default|GetActiveGamePlayTagContainer) "(TagName=\"AnimGaurd.AnimPlaying\")" true))
    (GameplayTags|AddGameplayTag (Variables|Default|GetActiveGamePlayTagContainer) "(TagName=\"AnimGaurd.AnimPlaying\")" :!class /Script/GameplayTags.BlueprintGameplayTagLibrary)
    (Animation|Montage|MontagePlay (Variables|Default|GetAnimInstance) _montagetoplay _inplayrate "MontageLength" 0.0 _stopallmontages)
    (Ability|Animation|MontageJumptoSection (Variables|Default|GetAnimInstance) _sectionname _montagetoplay)))

(event EventMontageStop
  (params (AnimMontage :type Anim%20Montage%20Object%20Reference))
  ;[0.15 0.15 0.15 0.5] Montage Funtion
  ;;[0.1308 0.15 0 0.5] Force Stop Montage
  (Animation|Montage|MontageStop (Variables|Default|GetAnimInstance) 0.1 AnimMontage))

(event EventAddTag
  (params (Tag :type Gameplay%20Tag%20Structure))
  (GameplayTags|AddGameplayTag (Variables|Default|GetActiveGamePlayTagContainer) Tag :!class /Script/GameplayTags.BlueprintGameplayTagLibrary))

(event EventRemoveTag
  (params (Tag :type Gameplay%20Tag%20Structure))
  (GameplayTags|RemoveGameplayTag (Variables|Default|GetActiveGamePlayTagContainer) Tag :!class /Script/GameplayTags.BlueprintGameplayTagLibrary))

(event EventSetSpeed
  (params (Speed :type Float%20%28double-precision%29))
  ;[0.15 0.15 0.15 0.5] Set Character Speed
  (Variables|/Script/Engine.CharacterMovementComponent|SetMaxWalkSpeed (Variables|Character|GetCharacterMovement) Speed))

(event Input|KeyboardEvents|DebugKeyU
  (params (Key :type Key%20Structure :default "None") (ActionValue :type Input%20Action%20Value%20Structure))
  (:Pressed
    (Variables|/Script/Engine.SpringArmComponent|SetSocketOffset (Variables|Default|GetCameraBoom) (+ (Variables|/Script/Engine.SpringArmComponent|GetSocketOffset (Variables|Default|GetCameraBoom)) "10.000000,0.000000,0.000000"))))

(event Input|KeyboardEvents|DebugKeyJ
  (params (Key :type Key%20Structure :default "None") (ActionValue :type Input%20Action%20Value%20Structure))
  (:Pressed
    (Variables|/Script/Engine.SpringArmComponent|SetSocketOffset (Variables|Default|GetCameraBoom) (+ (Variables|/Script/Engine.SpringArmComponent|GetSocketOffset (Variables|Default|GetCameraBoom)) "-10.000000,0.000000,0.000000"))))

(event Input|KeyboardEvents|DebugKeyK
  (params (Key :type Key%20Structure :default "None") (ActionValue :type Input%20Action%20Value%20Structure))
  (:Pressed
    (Variables|/Script/Engine.SpringArmComponent|SetSocketOffset (Variables|Default|GetCameraBoom) (+ (Variables|/Script/Engine.SpringArmComponent|GetSocketOffset (Variables|Default|GetCameraBoom)) "0.000000,10.000000,0.000000"))))

(event Input|KeyboardEvents|DebugKeyTab
  (params (Key :type Key%20Structure :default "None") (ActionValue :type Input%20Action%20Value%20Structure))
  ;[0.15 0.15 0.15 0.5] Global Time Dilation
  (:Pressed
    (Utilities|Time|SetGlobalTimeDilation 0.2))
  (:Released
    (Utilities|Time|SetGlobalTimeDilation 1.0)))

(event Input|KeyboardEvents|DebugKeyH
  (params (Key :type Key%20Structure :default "None") (ActionValue :type Input%20Action%20Value%20Structure))
  (:Pressed
    (Variables|/Script/Engine.SpringArmComponent|SetSocketOffset (Variables|Default|GetCameraBoom) (+ (Variables|/Script/Engine.SpringArmComponent|GetSocketOffset (Variables|Default|GetCameraBoom)) "10.000000,-10.000000,0.000000"))))

(event Input|KeyboardEvents|DebugKeyO
  (params (Key :type Key%20Structure :default "None") (ActionValue :type Input%20Action%20Value%20Structure))
  (:Pressed
    (Variables|/Script/Engine.SpringArmComponent|SetSocketOffset (Variables|Default|GetCameraBoom) (+ (Variables|/Script/Engine.SpringArmComponent|GetSocketOffset (Variables|Default|GetCameraBoom)) "0.000000,0.000000,10.000000"))))

(event Input|KeyboardEvents|DebugKeyL
  (params (Key :type Key%20Structure :default "None") (ActionValue :type Input%20Action%20Value%20Structure))
  (:Pressed
    (Variables|/Script/Engine.SpringArmComponent|SetSocketOffset (Variables|Default|GetCameraBoom) (+ (Variables|/Script/Engine.SpringArmComponent|GetSocketOffset (Variables|Default|GetCameraBoom)) "10.000000,0.000000,-10.000000"))))

(event Input|KeyboardEvents|DebugKeyI
  (params (Key :type Key%20Structure :default "None") (ActionValue :type Input%20Action%20Value%20Structure))
  (:Pressed
    (CallFunction|IAZoomingStarted)))

(fn ConstructionScript)

(fn PlayMovementAnim
  (params (StartMontage :type Boolean) (ForwardDirection :type Integer) (RightDirection :type Integer))
  (bind _as_abp_character_rifle (Variables|Default|GetAs%20ABP%20Character%20Rifle))
  (bind _enum_direction (Default|SetDirectionEnum _as_abp_character_rifle (Variables|/Game/AnimationsHud/EnemyAnim/ABP_CharacterRifle.ABP_CharacterRifle_C|GetDirection _as_abp_character_rifle) ForwardDirection RightDirection))
  (CallFunction|PlayAnimation))

(fn TagBatchDelete
  (params (TagTwo :type Gameplay%20Tag%20Structure))
  (for _array_element (GameplayTags|BreakGameplayTagContainer (Variables|Default|GetActiveGamePlayTagContainer))
    (if (GameplayTags|MatchesTag _array_element TagTwo)
      (GameplayTags|RemoveGameplayTag (Variables|Default|GetActiveGamePlayTagContainer) _array_element :!class /Script/GameplayTags.BlueprintGameplayTagLibrary)))
  (return true))

(fn SwitchMode
  (bind _activegameplaytagcontainer (Variables|Default|GetActiveGamePlayTagContainer))
  (if (!= (Variables|Default|GetLoopCounterForRifilingMode) (Variables|Default|GetMaxLoopCounter))
    (Variables|Default|SetLoopCounterForRifilingMode (+ (Variables|Default|GetLoopCounterForRifilingMode) 1))
    (else
      (Variables|Default|SetLoopCounterForRifilingMode 0)))
  (switch int (Variables|Default|GetLoopCounterForRifilingMode)
    (:0
      (GameplayTags|AddGameplayTag _activegameplaytagcontainer "(TagName=\"FiringMode.Auto\")" :!class /Script/GameplayTags.BlueprintGameplayTagLibrary))
    (:1
      (GameplayTags|AddGameplayTag _activegameplaytagcontainer "(TagName=\"FiringMode.Brust\")" :!class /Script/GameplayTags.BlueprintGameplayTagLibrary))
    (:2
      (GameplayTags|AddGameplayTag _activegameplaytagcontainer "(TagName=\"FiringMode.Single\")" :!class /Script/GameplayTags.BlueprintGameplayTagLibrary))))

(fn GetSpawnTransFormLocationRotation
  (bind _mesh (Variables|Character|GetMesh))
  (bind _followcamera (Variables|Default|GetFollowCamera))
  (bind _returnvalue (Transformation|GetSocketLocation _mesh "hand_Granade"))
  (bind _returnvalue_2 (+ _returnvalue "50.000000,0.000000,0.000000"))
  (return _returnvalue_2 (Math|Rotator|FindLookatRotation _returnvalue_2 (+ (Transformation|GetWorldLocation _followcamera) (* (Math|Rotator|GetRotationXVector (Transformation|GetWorldRotation _followcamera)) 5e+03)))))

(fn GetGamePlayTagContainer
  (return (Variables|Default|GetActiveGamePlayTagContainer)))

(fn GetLeftIKTransform
  (bind _weapon (Variables|Default|GetWeapon))
  (bind _mesh (Variables|Character|GetMesh))
  (bind _gunskeletalmesh (Variables|/Game/Main/Wepon/Gun/Base_Gun.Base_Gun_C|GetGunSkeletalMesh _weapon))
  (bind _returnvalue (Transformation|GetSocketTransform _gunskeletalmesh "LeftHand_IK" "RTS_World"))
  (bind (_outposition _outrotation) (Class|SkinnedMeshComponent|TransformtoBoneSpace _mesh "hand_r" (.location _returnvalue) (.rotation _returnvalue)))
  (Utilities|IsValid _weapon
    (:Is%20Valid
      (return (Math|Transform|MakeTransform _outposition _outrotation)))))

(fn GetActiveGamePlayTagContainer
  (return (Variables|Default|GetActiveGamePlayTagContainer)))

(fn GetCharacter
  (return self))