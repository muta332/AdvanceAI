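; Enemy character Blueprint that spawns a gun into its right-hand socket and plays rifle fire montages on attack input.
; Pressing attack fires once, then repeats by looping timer in Automatic or by loop in Brust (burst) mode; releasing clears the timer and stops the montage.
; A shared PlayAnim helper plays montage sections, including directional start/stop movement montages, though that movement path is disconnected from its empty event.
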(event Custom|ExecuteAttack
  (CallFunction|PlayAnim "/Game/AnimationsHud/_FixedRifle/Fire/AM_FireSequence.AM_FireSequence" "None" (Variables|Default|GetAnimSpeed)))

(event Input|EnhancedActionEvents|EnhancedInputActionIA_Attack
  (params (ActionValue :type Boolean) (ElapsedSeconds :type Float%20%28double-precision%29) (TriggeredSeconds :type Float%20%28double-precision%29) (InputAction :type Input%20Action%20Object%20Reference :default "/Game/ThirdPerson/Input/Actions/IA_Attack.IA_Attack"))
  (:Started
    (if true
      (CallFunction|ExecuteAttack)
      (switch Utilities|FlowControl|Switch|SwitchonE_FiringMode (Variables|Default|GetE_RifleMode)
        (:NewEnumerator0
          (bind _returnvalue (Utilities|Time|SetTimerbyFunctionName 0 "ExecuteAttack" (Variables|Default|GetBulletRate) true))
          (Variables|Default|SetAttackTimer _returnvalue))
        (:NewEnumerator1
          (Utilities|FlowControl|DoOnce false :!label _label
            (:Completed
              (for _index (range 1 (Variables|Default|GetbrustFireRate))
                (CallFunction|ExecuteAttack)
                (Development|PrintString "Hello" true true "(R=0.000000,G=0.660000,B=1.000000,A=1.000000)" 2.0 "2"))
              (goto _label Reset)))))))
  (:Completed
    (Utilities|FlowControl|Sequence
      (:then_0
        (goto _label Reset))
      (:then_1
        (Utilities|Time|ClearandInvalidateTimerbyHandle (Variables|Default|GetAttackTimer))
        (Animation|Montage|MontageStop (Components|SkeletalMesh|GetAnimInstance (Variables|Character|GetMesh)) 0.0 "/Game/AnimationsHud/_FixedRifle/Fire/AM_FireSequence.AM_FireSequence")))))

(event EventBeginPlay
  (bind _mesh (Variables|Character|GetMesh))
  (bind _returnvalue (Game|SpawnActorfromClass "/Game/Main/Wepon/Gun/AR/Gun.Gun_C" (Math|Transform|MakeTransform "0, 0, 0" "0, 0, 0" "1.000000,1.000000,1.000000") "Undefined" "MultiplyWithRoot" 0 0))
  (Transformation|AttachComponentToComponent _returnvalue _mesh "hand_rSocket" "SnapToTarget" "SnapToTarget" "SnapToTarget" true)
  (bind _asabp_character_rifle (Utilities|Casting|CastToABP_CharacterRifle (Components|SkeletalMesh|GetAnimInstance _mesh)))
  (Variables|Default|SetAs%20ABP%20Character%20Rifle _asabp_character_rifle))

(event EventPlayMovementAnimation
  (params (StartMontage :type Boolean) (ForwardDirection :type Integer) (RightDirection :type Integer)))

(fn ConstructionScript)

(fn PlayMovementAnim
  (params (StartMontage :type Boolean) (ForwardDirection :type Integer) (RightDirection :type Integer))
  (bind _as_abp_character_rifle (Variables|Default|GetAs%20ABP%20Character%20Rifle))
  (bind _enum_direction (Default|SetDirectionEnum _as_abp_character_rifle (Variables|/Game/AnimationsHud/EnemyAnim/ABP_CharacterRifle.ABP_CharacterRifle_C|GetDirection _as_abp_character_rifle) ForwardDirection RightDirection))
  (CallFunction|PlayAnim (select StartMontage "/Game/AnimationsHud/_FixedRifle/Run/RunStart/LFoot/AM_StartMontage.AM_StartMontage" "/Game/AnimationsHud/_FixedRifle/Run/RunStop/WorkingRunToStop/AM_StopMontage.AM_StopMontage") (Utilities|Select :Index _enum_direction :NewEnumerator0 "Forward" :NewEnumerator1 "BackWard" :NewEnumerator2 "ForwardLeft" :NewEnumerator3 "Left" :NewEnumerator4 "BackWardLeft" :NewEnumerator5 "ForwardRight" :NewEnumerator6 "Right" :NewEnumerator7 "BackWardRight") 0.0)
  (Development|PrintString (Utilities|String|ToString(Name) (Utilities|Select :Index _enum_direction :NewEnumerator0 "Forward" :NewEnumerator1 "BackWard" :NewEnumerator2 "ForwardLeft" :NewEnumerator3 "Left" :NewEnumerator4 "BackWardLeft" :NewEnumerator5 "ForwardRight" :NewEnumerator6 "Right" :NewEnumerator7 "BackWardRight"))))

(fn PlayAnim
  (params (MontageToPlay :type Anim%20Montage%20Object%20Reference) (SectionName :type Name) (InPlayRate :type Float%20%28single-precision%29))
  (bind _mesh (Variables|Character|GetMesh))
  (bind _returnvalue (Components|SkeletalMesh|GetAnimInstance _mesh))
  (Animation|Montage|MontagePlay _returnvalue MontageToPlay InPlayRate "MontageLength" 0.0 true)
  (Ability|Animation|MontageJumptoSection _returnvalue SectionName MontageToPlay))