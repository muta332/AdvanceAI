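; Player character that spawns a weapon attached to its mesh and forwards trigger, reload and fire-mode input to a gun system.
; Stance changes are tracked in a gameplay tag container and set walk speed, with crouch blocking sprint and run requests.
; Gun fire events freeze and restore movement.
; It also plays montages and clears the shooting tag on completion, though the RemoveTag event actually adds its tag.
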(event OnFireStarted(GunSystem)
  ;[0.15 0.15 0.15 0.5] On Fire Start and End
  (CallFunction|SetSpeed 0.0)
  (Pawn|Components|CharacterMovement|SetMovementMode (Variables|Character|GetCharacterMovement) "MOVE_None" 0))

(event OnFireEnded(GunSystem)
  ;[0.15 0.15 0.15 0.5] On Fire Start and End
  (Pawn|Components|CharacterMovement|SetMovementMode (Variables|Character|GetCharacterMovement) "MOVE_Walking" 0)
  (CallFunction|RemoveTag "(TagName=\"Status.Shooting\")")
  (if (not (GameplayTags|HasTag (Variables|Default|GetActiveGamePlayTagContainer) "(TagName=\"Stance.Crouching\")"))
    (CallFunction|SetSpeed (Variables|Default|GetMax%20Run%20speed))
    (else
      (CallFunction|SetSpeed (Variables|Default|GetMax%20Crouch/Walk%20Speed)))))

(event Custom|StanceChangeSprint
  ;[0.15 0.1168 0 0.5] StanceChange
  (if (not (GameplayTags|HasTag (Variables|Default|GetActiveGamePlayTagContainer) "(TagName=\"Stance.Crouching\")"))
    (CallFunction|OnStanceChange "(TagName=\"Stance.Sprinting\")")))

(event Custom|StanceChangeRunning
  ;[0.15 0.1168 0 0.5] StanceChange
  (if (not (GameplayTags|HasTag (Variables|Default|GetActiveGamePlayTagContainer) "(TagName=\"Stance.Crouching\")"))
    (CallFunction|OnStanceChange "(TagName=\"Stance.Running\")")))

(event Custom|GunTrigger
  ;[0.15 0.15 0.15 0.5] GunTrigger
  (Default|Triggered (Variables|Default|GetGunSystem)))

(event Custom|GunTriggerEnd
  ;[0.15 0.15 0.15 0.5] GunTrigger
  (Default|TriggerReleased (Variables|Default|GetGunSystem)))

(event Custom|Reloading
  ;[0.15 0.15 0.15 0.5] GunTrigger
  (Default|Reloading (Variables|Default|GetGunSystem)))

(event Custom|StanceChangeWalking
  ;[0.15 0.1168 0 0.5] StanceChange
  (Utilities|FlowControl|FlipFlop
    (:A
      (CallFunction|OnStanceChange "(TagName=\"Stance.Walking\")"))
    (:B
      (CallFunction|OnStanceChange "(TagName=\"Stance.Running\")"))))

(event Custom|Switch%20GunMode
  (Default|SwtichFiringMode (Variables|Default|GetGunSystem)))

(event Custom|Spawn%20Primary%20Weapon
  (params (Class :type Gun%20Class%20Reference))
  (bind _self self)
  ;[0.15 0.15 0.15 0.5] Weapon
  (bind _returnvalue (Game|SpawnActorfromClass Class (Math|Transform|MakeTransform "0, 0, 0" "0, 0, 0" "1.000000,1.000000,1.000000") "Undefined" "MultiplyWithRoot" _self _self))
  (bind _output_get (Variables|Default|SetWeapon _returnvalue))
  (Transformation|AttachComponentToComponent _output_get (Variables|Character|GetMesh) (Variables|Default|GetAttachWeaponToSocket) "SnapToTarget" "SnapToTarget" "SnapToTarget" true))

(event Custom|Funtion%20Binding
  ;[0.15 0.15 0.15 0.5] Bind Events
  (EventDispatchers|AssignOnMontageEnded (Variables|Default|GetAnimInstance) (EventDispatchers|CreateEvent :!event Custom|OnMontageEnded_Event)))

(event Custom|OnMontageEnded_Event
  (params (Montage :type Anim%20Montage%20Object%20Reference) (bInterrupted :type Boolean))
  ;[0.15 0.15 0.15 0.5] Montage Funtion
  ;;[0.15 0.01724 0 0.5] MontageEnd or Interrupt
  (if (not bInterrupted)
    (GameplayTags|RemoveGameplayTag (Variables|Default|GetActiveGamePlayTagContainer) "(TagName=\"Status.Shooting\")" :!class /Script/GameplayTags.BlueprintGameplayTagLibrary)))

(event Custom|StanceCrouching
  ;[0.15 0.1168 0 0.5] StanceChange
  (Utilities|FlowControl|FlipFlop
    (:A
      (CallFunction|OnStanceChange "(TagName=\"Stance.Crouching\")"))
    (:B
      (CallFunction|OnStanceChange "(TagName=\"Stance.Running\")"))))

(event Custom|On%20Stance%20Change
  (params (Stance%20Tag :type Gameplay%20Tag%20Structure))
  (bind _activegameplaytagcontainer (Variables|Default|GetActiveGamePlayTagContainer))
  ;[0.15 0.15 0.15 0.5] Stance Change
  (CallFunction|TagBatchDelete "(TagName=\"Stance\")")
  (|SwitchGameplayTag Stance%20Tag
    (:Stance.Crouching
      (GameplayTags|AddGameplayTag _activegameplaytagcontainer "(TagName=\"Stance.Crouching\")" :!class /Script/GameplayTags.BlueprintGameplayTagLibrary)
      (CallFunction|SetSpeed (Variables|Default|GetMax%20Crouch/Walk%20Speed)))
    (:Stance.Running
      (GameplayTags|AddGameplayTag _activegameplaytagcontainer "(TagName=\"Stance.Running\")" :!class /Script/GameplayTags.BlueprintGameplayTagLibrary)
      (CallFunction|SetSpeed (Variables|Default|GetMax%20Run%20speed)))
    (:Stance.Sprinting
      (GameplayTags|AddGameplayTag _activegameplaytagcontainer "(TagName=\"Stance.Sprinting\")" :!class /Script/GameplayTags.BlueprintGameplayTagLibrary)
      (CallFunction|SetSpeed (Variables|Default|GetMax%20Sprint%20Speed)))
    (:Stance.Walking
      (GameplayTags|AddGameplayTag _activegameplaytagcontainer "(TagName=\"Stance.Walking\")" :!class /Script/GameplayTags.BlueprintGameplayTagLibrary)
      (CallFunction|SetSpeed (Variables|Default|GetMax%20Crouch/Walk%20Speed)))))

(event EventAddTag
  (params (Tag :type Gameplay%20Tag%20Structure))
  (GameplayTags|AddGameplayTag (Variables|Default|GetActiveGamePlayTagContainer) Tag :!class /Script/GameplayTags.BlueprintGameplayTagLibrary))

(event EventBeginPlay
  (CallFunction|FuntionBinding)
  (CallFunction|SpawnPrimaryWeapon "/Game/Main/Wepon/Gun/AR/Gun.Gun_C"))

(event EventPlayAnimation
  (params (AnimMontageStuct :type Struct%20Montage%20Structure))
  (bind (_montagetoplay _inplayrate _sectionname _stopallmontages) (Utilities|Struct|BreakStruct_Montage AnimMontageStuct))
  ;[0.15 0.15 0.15 0.5] Montage Funtion
  ;;[0 0.15 0.1298 0.5] Montage Begin
  (Animation|Montage|MontagePlay (Variables|Default|GetAnimInstance) _montagetoplay _inplayrate "MontageLength" 0.0 _stopallmontages)
  (Ability|Animation|MontageJumptoSection (Variables|Default|GetAnimInstance) _sectionname 0))

(event EventMontageStop
  (params (AnimMontage :type Anim%20Montage%20Object%20Reference))
  ;[0.15 0.15 0.15 0.5] Montage Funtion
  ;;[0.1308 0.15 0 0.5] Force Stop Montage
  (Animation|Montage|MontageStop (Variables|Default|GetAnimInstance) 0.1 AnimMontage))

(event EventSetSpeed
  (params (Speed :type Float%20%28double-precision%29))
  (Variables|/Script/Engine.CharacterMovementComponent|SetMaxWalkSpeed (Variables|Character|GetCharacterMovement) Speed))

(event EventRemoveTag
  (params (Tag :type Gameplay%20Tag%20Structure))
  (GameplayTags|AddGameplayTag (Variables|Default|GetActiveGamePlayTagContainer) Tag :!class /Script/GameplayTags.BlueprintGameplayTagLibrary))

(fn ConstructionScript)

(fn TagBatchDelete
  (params (Parent%20Tag :type Gameplay%20Tag%20Structure))
  (for _array_element (GameplayTags|BreakGameplayTagContainer (Variables|Default|GetActiveGamePlayTagContainer))
    (if (GameplayTags|MatchesTag _array_element Parent%20Tag)
      (CallFunction|RemoveTag)))
  (return true))

(fn GetGamePlayTagContainer
  (return ""))

(fn GetActiveGamePlayTagContainer
  (return (Variables|Default|GetActiveGamePlayTagContainer)))