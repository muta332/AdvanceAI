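; A grenade projectile actor that bounces and explodes with sound and particle effects.
; When its projectile tick flag is set, BeginPlay configures launch speed, gravity and collision and starts a fuse timer, one tick after spawning.
; Bounce sounds are capped with a DoN.
; The blast sphere-traces for pawns and soon expires the actor; hits only feed an optional debug print, with no damage applied.
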(event Custom|GranadeBlast
  (bind _returnvalue (Transformation|GetActorLocation))
  (Actor|SetLifeSpan 0.1)
  (bind _outhits (Collision|MultiSphereTraceForObjects (Transformation|GetActorLocation) (Transformation|GetActorLocation) 5e+02 (Utilities|Array|MakeArray "ObjectTypeQuery3") false 0 (select (Variables|Default|GetDrawBlastSphere) "ForDuration" "None")))
  (Audio|PlaySoundatLocation "/Game/Main/Wepon/Granade/Sounds/MS_GranadeBlast.MS_GranadeBlast" _returnvalue "0, 0, 0" 1.0 1.0 0.0 0 0 0 0)
  (Effects|SpawnEmitteratLocation "/Game/StarterContent/Particles/P_Explosion.P_Explosion" _returnvalue "0, 0, 0" (* "1.000000,1.000000,1.000000" 7.0))
  (for _array_element _outhits
    (Utilities|FlowControl|Sequence
      (:then_1
        (if (Variables|Default|GetPrintDebugBlastHitNames)
          (Development|PrintString (Utilities|GetDisplayName (.HitActor (Collision|BreakHitResult _array_element)))))))))

(event Custom|OnProjectileBounce_Event
  (params (ImpactResult :type Hit%20Result%20Structure%20%28by%20ref%29) (ImpactVelocity :type Vector%20%28by%20ref%29))
  (Utilities|FlowControl|DoN 4
    (:Exit
      (Audio|PlaySoundatLocation "/Game/Main/Wepon/Granade/Sounds/MS_GranadeBounce.MS_GranadeBounce" (Transformation|GetActorLocation) "0, 0, 0" 1.0 1.0 0.0 0 0 0 0))))

(event Custom|BindFunctions
  (EventDispatchers|AssignOnProjectileBounce (Variables|Default|GetProjectileMovement) (EventDispatchers|CreateEvent :!event Custom|OnProjectileBounce_Event)))

(event EventBeginPlay
  (bind _projectilecomponenttickenabled (Variables|Default|GetProjectileComponentTickEnabled))
  (bind _projectilemovement (Variables|Default|GetProjectileMovement))
  (bind _granade (Variables|Default|GetGranade))
  (Utilities|FlowControl|DelayUntilNextTick)
  (CallFunction|BindFunctions)
  (Components|Tick|SetComponentTickEnabled (Variables|Default|GetProjectileMovement) _projectilecomponenttickenabled)
  (if _projectilecomponenttickenabled
    (Utilities|Time|SetTimerbyEvent (EventDispatchers|CreateEvent :!event Custom|GranadeBlast) 4.0)
    (Variables|/Script/Engine.ProjectileMovementComponent|SetInitialSpeed _projectilemovement (Variables|Default|GetInitial%20Speed))
    (Variables|/Script/Engine.ProjectileMovementComponent|SetProjectileGravityScale _projectilemovement (Variables|Default|GetProjectileGravity))
    (Collision|SetCollisionEnabled _granade "QueryAndPhysics")
    (Collision|SetCollisionResponsetoChannel _granade "ECC_WorldStatic" "ECR_Block")))

(fn ConstructionScript)