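; Interactable ammo storage that supplies ammo to the interacting character's weapon.
; On Interact it runs the parent logic, gets the character's weapon through GetCharacterMessage and passes a set amount to its GunSystem via SetAmmoStorage.
; It then subtracts that amount from its remaining ammo, with no empty check here.
; GetInteractText keeps the parent prompt and adds a remaining-ammo label.
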(event EventBeginPlay)

(event Collision|EventActorBeginOverlap
  (params (OtherActor :type Actor%20Object%20Reference)))

(event EventInteract
  (params (Instigator :type Actor%20Object%20Reference))
  (bind _increase_ammo_storage_ammount (Variables|Default|GetIncrease%20Ammo%20Storage%20Ammount))
  (|CallParentFunction Instigator)
  (bind _character (Class|BPICharacterInterface|GetCharacter(Message) Instigator))
  (Default|SetAmmoStorage (Actor|GetComponentbyClass (Variables|/Game/Main/Player/BP_Player.BP_Player_C|GetWeapon _character) "/Game/Main/GunSystem/GunSystem.GunSystem_C") _increase_ammo_storage_ammount)
  (Variables|Default|SetRemainig%20Ammo%20 (- (Variables|Default|GetRemainig%20Ammo%20) _increase_ammo_storage_ammount)))

(event EventTick
  (params (DeltaSeconds :type Float%20%28single-precision%29)))

(fn ConstructionScript)

(fn GetInteractText
  (bind _text (|CallParentFunction))
  (return _text (Utilities|Text|ToText(String) (Utilities|String|Append "Remaining Ammo" "         " (Utilities|String|ToString(Integer) (Variables|Default|GetRemainig%20Ammo%20))))))