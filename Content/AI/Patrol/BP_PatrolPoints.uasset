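; Patrol path actor that hands out world-space spline points as successive patrol destinations, presumably for AI.
; BeginPlay caches the spline's point count as MaxPoints.
; Each FindNextSplineLocation call steps CurrentPoints by Incrementor, which flips at MaxPoints or MinimumPoints to ping-pong along the path.
; The upper flip compares against the point count, so the index reaches one past the last point.
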(event EventBeginPlay
  (Variables|Default|SetMaxPoints (CallFunction|GetTotalPatrolPoints)))

(fn ConstructionScript)

(fn GetTotalPatrolPoints
  (return (Spline|GetNumberOfSplinePoints (Variables|Default|GetSpline))))

(fn FindNextSplineLocation
  (CallFunction|CalculateSpline)
  (return (Spline|GetLocationatSplinePoint (Variables|Default|GetSpline) (Variables|Default|GetCurrentPoints) "World")))

(fn NewFunction)

(fn CalculateSpline
  (Variables|Default|SetCurrentPoints (+ (Variables|Default|GetCurrentPoints) (Variables|Default|GetIncrementor)))
  (if (>= (Variables|Default|GetCurrentPoints) (Variables|Default|GetMaxPoints))
    (Variables|Default|SetIncrementor -1)
    (elif (<= (Variables|Default|GetCurrentPoints) (Variables|Default|GetMinimumPoints))
      (Variables|Default|SetIncrementor 1))))