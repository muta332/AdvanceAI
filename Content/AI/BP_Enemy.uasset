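; Base enemy AI character that uses gameplay tags for stance speeds, gun identification, target visibility and a defensive state on low health.
; A hostile target starts a looping timer that line-traces to it and toggles the EnemyVisible tag.
; The health component feeds an on-screen health bar, created on demand, and damage type selects the hit-reaction montage.
; It also triggers grenade throws and supplies patrol spline points; several combat getters are stubs.
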(event OnLowonHealth(HealthAndDamageSystem)
  (params (DamageCauser :type Actor%20Object%20Reference) (Health :type Float%20%28single-precision%29))
  (Class|GamePlayTagInterFaces|AddTag "(TagName=\"AICommand.Diffence\")")
  (Default|CallOnLowHealth DamageCauser Health self))

(event OnHealed(HealthAndDamageSystem)
  (params (Health :type Float%20%28single-precision%29) (MaxHealth :type Float%20%28single-precision%29))
  (Class|GEnemyPopUpWidget|SetPercent (Variables|Default|GetAttachedPlayerWidget) Health MaxHealth))

(event Custom|Start%20Granade
  (Default|GranadeStart (Variables|Default|GetGranadeSystem) (Utilities|Struct|MakeStruct_GAS_System 0 self "(TagName=\"\")" true)))

(event Custom|ThrowGranade
  (Default|ReleaseInput (Variables|Default|GetGranadeSystem)))

(event Custom|Debugger
  (bind _returnvalue (Actor|GetActorOfClass "/Game/Main/Player/BP_Player.BP_Player_C"))
  (AI|Components|Blackboard|SetValueasObject (AI|GetBlackboard (AI|GetAIController self)) (Utilities|Name|MakeLiteralName "EnemyActor") _returnvalue))

(event Custom|Update%20Percet
  (bind _ghealthanddamagesystem (Variables|Default|GetGHealthAndDamageSystem))
  (Default|SetPercent (Variables|Default|GetAttachedPlayerWidget) (Variables|/Script/AdvanceAI.GHealthAndDamageSystem|GetHealth _ghealthanddamagesystem) (Variables|/Script/AdvanceAI.GHealthAndDamageSystem|GetMaxHealth _ghealthanddamagesystem)))

(event Custom|PlayDamageResponseAnim
  (bind _animmontage (Variables|Default|GetAnimMontage))
  (if (not (<= (Variables|/Script/AdvanceAI.GHealthAndDamageSystem|GetHealth (Variables|Default|GetGHealthAndDamageSystem)) 0.0))
    (Class|GCharacterInterface|PlayAnimation(Message) self (Utilities|Select :Index (Variables|Default|GetDamageType) :EDT_None "" :EDT_Projectile (.Value (Utilities|Map|Find _animmontage "(TagName=\"Animation.ProjectileDamageReaction\")")) :EDT_Explosion (.Value (Utilities|Map|Find _animmontage "(TagName=\"Animation.ExplosionReaction\")")) :EDT_Environment "" :EDT_Melee (.Value (Utilities|Map|Find _animmontage "(TagName=\"Animation.MeleeDamageReaction\")"))))))

(event Custom|HealthWidgetOnDamageResponse
  (params (DamageType :type EDamageType%20Enum :default "EDT_None") (DamageCauser :type Object%20Object%20Reference))
  (bind _returnvalue (Game|GetPlayerController 0))
  (Variables|Default|SetDamageType DamageType)
  (Variables|Default|GetAttachedPlayerWidget
    (:then)
    (:else
      ;[0.15 0.15 0.15 0.5] Target has to be player since widget used for player
      (bind _returnvalue_2 (Class|GCharacterInterface|CheckifHostile(Message) DamageCauser self))
      (bind _returnvalue_3 (UserInterface|CreateWidget "/Game/Main/PlayerWidget/WBP_AIHealth.WBP_AIHealth_C" _returnvalue self _returnvalue 1.3e+02 _returnvalue_2))
      (bind _output_get (Variables|Default|SetAttachedPlayerWidget _returnvalue_3))
      (UserInterface|Viewport|AddtoViewport _output_get 0))))

(event EventSetTargetActor
  (params (TargetActor :type Actor%20Object%20Reference))
  (bind _returnvalue (Class|GCharacterInterface|CheckifHostile(Message) self TargetActor))
  (if _returnvalue
    (Variables|Default|SetTargetActor TargetActor)
    (Utilities|Time|SetTimerbyFunctionName 0 "TargetActorVisible" 0.1 true)))

(event EventBeginPlay
  (Class|GamePlayTagInterFaces|AddTag (Variables|Default|GetGunIdentificationTag)))

(event EventOnFireEndedEvent
  (Variables|/Game/Attack/BPC_Attacks.BPC_Attacks_C|SetAutoFiringCounter (Variables|Default|GetBPC_Attacks) 0))

(event EventSetSpeedBasedonStanceTag
  (params (StanceTag :type Gameplay%20Tag%20Structure))
  (|SwitchGameplayTag StanceTag
    (:Stance.Crouching
      (Class|GCharacterInterface|SetSpeed (Variables|Default|GetCrouchAndWalkSpeed)))
    (:Stance.Running
      (Class|GCharacterInterface|SetSpeed (Variables|Default|GetMaxRunSpeed)))
    (:Stance.Sprinting
      (Class|GCharacterInterface|SetSpeed (Variables|Default|GetMaxSprintSpeed)))
    (:Stance.Walking
      (Class|GCharacterInterface|SetSpeed (Variables|Default|GetCrouchAndWalkSpeed)))))

(fn ConstructionScript
  (bind _ghealthanddamagesystem (Variables|Default|GetGHealthAndDamageSystem))
  (EventDispatchers|BindEventtoOnDamageResponse _ghealthanddamagesystem (EventDispatchers|CreateEvent :!event OnDamageResponse))
  (EventDispatchers|BindEventtoOnDeath _ghealthanddamagesystem (EventDispatchers|CreateEvent :!event OnDeath)))

(fn GetSpeed
  (params (StanceTag :type Gameplay%20Tag%20Structure%20%28by%20ref%29))
  (|SwitchGameplayTag StanceTag
    (:Stance.Crouching
      (Class|GCharacterInterface|SetSpeed (Variables|Default|GetCrouchAndWalkSpeed)))
    (:Stance.Running
      (Class|GCharacterInterface|SetSpeed (Variables|Default|GetMaxRunSpeed)))
    (:Stance.Sprinting
      (Class|GCharacterInterface|SetSpeed (Variables|Default|GetMaxSprintSpeed)))
    (:Stance.Walking
      (Class|GCharacterInterface|SetSpeed (Variables|Default|GetCrouchAndWalkSpeed)))))

(fn TargetActorVisible
  (Utilities|Array|Clear (LocalVariables|GetActorsToIgonore))
  (bind _targetactor (Variables|Default|GetTargetActor)
    (:then
      (bind _outhits (Collision|MultiLineTraceByChannel (Transformation|GetActorLocation) (Transformation|GetActorLocation _targetactor) "TraceTypeQuery1" false (LocalVariables|GetActorsToIgonore) "None"))
      (for _array_element _outhits
        (if (== (.HitActor (Collision|BreakHitResult _array_element)) (Variables|Default|GetTargetActor))
          (Class|GamePlayTagInterFaces|AddTag "(TagName=\"EnemyVisible\")")
          (else
            (Class|GamePlayTagInterFaces|RemoveTag "(TagName=\"EnemyVisible\")")))))
    (:else)))

(fn ReserveAttackToken
  (params (Amount :type Integer))
  (return false))

(fn IsAttacking
  (return false))

(fn IsDead
  (return false))

(fn GetMaxHealth
  (return 0.0))

(fn GetCurrentHealth
  (return 0.0))

(fn TakeDamage
  (params (DamageInfo :type Damage%20Info%20Structure%20%28by%20ref%29))
  (bind _self self)
  (bind _returnvalue (Utilities|GetDisplayName _self))
  (bind _returnvalue_2 (|CallParentFunction DamageInfo))
  (Development|PrintString (Utilities|String|Append _returnvalue "=" (Utilities|String|ToString(Float) (Variables|/Script/AdvanceAI.GHealthAndDamageSystem|GetHealth (Variables|Default|GetHealthAndDamageSystem)))) true true "(R=0.000000,G=0.660000,B=1.000000,A=1.000000)" 2.0 (Utilities|String|StringToName _returnvalue))
  (return _returnvalue_2))

(fn GetGunIdentificationTagName
  (return (Variables|Default|GetGunIdentificationTag)))

(fn GetSplineLocation
  (bind _bp_patrol (Variables|Default|GetBP_Patrol))
  (Utilities|IsValid _bp_patrol
    (:Is%20Valid
      (bind _location (Default|FindNextSplineLocation _bp_patrol))
      (return _location))
    (:Is%20Not%20Valid
      (Development|PrintString (Utilities|String|Append (Utilities|GetDisplayName self) ": Spline Not Valid. Set the Spline in World") true true "(R=1.000000,G=0.141862,B=0.000000,A=1.000000)" 1e+01 "Spline"))))

(fn GetTargetActor
  (bind _targetactor (Variables|Default|GetTargetActor))
  (Utilities|IsValid _targetactor
    (:Is%20Valid
      (return _targetactor))))