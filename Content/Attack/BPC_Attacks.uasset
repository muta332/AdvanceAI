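; Attack component that handles projectile, melee and area-of-effect damage plus camera lock-in on a target.
; Projectiles aim at the first line-trace hit, spread as the shot count grows, damage hostiles on impact, and let targeted enemies attempt a block.
; Melee runs looping timer sphere traces along the weapon; AOE spawns an actor that damages overlaps.
; Lock-in toggles a camera-forward sphere-trace target that Tick turns the controller toward.
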(event Custom|LockTrace
  ;[0.15 0.15 0.15 0.5] Lock In functionaliy
  (CallFunction|SetLockinActor))

(event Custom|OnComponentHit_Event
  (params (HitComponent :type Primitive%20Component%20Object%20Reference) (OtherActor :type Actor%20Object%20Reference) (OtherComp :type Primitive%20Component%20Object%20Reference) (NormalImpulse :type Vector) (Hit :type Hit%20Result%20Structure%20%28by%20ref%29))
  (bind _returnvalue (Components|GetOwner))
  (bind _returnvalue_2 (Components|GetOwner))
  (bind _returnvalue_3 (Components|GetOwner))
  (bind _projectile_info (Variables|Default|GetProjectile%20Info))
  (bind _projectile_info_2 (Variables|Default|GetProjectile%20Info))
  (bind (_destroyedemitter _destroyedemitterscale) (Utilities|Struct|BreakProjectileInfo _projectile_info_2))
  (bind _damageinfo (Utilities|Struct|BreakProjectileInfo _projectile_info))
  ;[0.15 0.15 0.15 0.5] On Enemy Hit with Projectile
  (Effects|SpawnEmitteratLocation _destroyedemitter (Transformation|GetWorldLocation HitComponent) "0, 0, 0" (* 1.0 _destroyedemitterscale))
  (bind _returnvalue_4 (Class|GCharacterInterface|CheckifHostile(Message) _returnvalue OtherActor))
  (if (and (!= _returnvalue HitComponent) _returnvalue_4)
    (Class|AISenseDamage|ReportDamageEvent OtherActor _returnvalue_2 0.0 (Transformation|GetActorLocation _returnvalue_2) "0, 0, 0" "None")
    (Class|GCharacterInterface|TakeDamage(Message) OtherActor _damageinfo)
    (Class|AISenseDamage|ReportDamageEvent OtherActor _returnvalue_3 (Utilities|Struct|BreakDamageInfo _damageinfo) (Transformation|GetActorLocation _returnvalue_3) (Transformation|GetActorLocation OtherActor) "None")
    (Actor|DestroyActor (Components|GetOwner HitComponent))
    (else
      (Actor|DestroyActor (Components|GetOwner HitComponent)))))

(event Custom|AOE%20Overlap
  (params (Actor :type Actor%20Object%20Reference))
  ;[0.15 0.15 0.15 0.5] on Aoe trace Overlap
  (Class|BPIDamagable|TakeDamage(Message) Actor (Utilities|Struct|BreakStruct_AOE (Variables|Default|GetAOE%20Info)) (Components|GetOwner))
  (Utilities|FlowControl|DelayUntilNextTick)
  (Actor|SetLifeSpan (Variables|Default|GetAOE%20Actor) 0.1))

(event Custom|Trace
  (bind _returnvalue (Components|GetOwner))
  ;[0.15 0.15 0.15 0.5] Sword Trace Logic
  (bind (_outhits _returnvalue_2) (Collision|MultiSphereTraceForObjects (Transformation|GetWorldLocation (Variables|/Game/Main/Wepon/BP_BaseMelee.BP_BaseMelee_C|GetStartTracePosition (stale Custom|Weapon%20Trace%20Start _asbp_base_melee))) (Transformation|GetWorldLocation (Variables|/Game/Main/Wepon/BP_BaseMelee.BP_BaseMelee_C|GetEndTracePosition (stale Custom|Weapon%20Trace%20Start _asbp_base_melee))) (stale Custom|Weapon%20Trace%20Start Radius) (Variables|Default|GetObject%20Types) false (Variables|Default|GetActors%20to%20Ignore) "None"))
  (for _array_element _outhits
    (if _returnvalue_2
      (Utilities|Array|AddUnique (Variables|Default|GetActors%20to%20Ignore) (.HitActor (Collision|BreakHitResult _array_element)))
      (bind _returnvalue_3 (Class|GCharacterInterface|CheckifHostile(Message) _returnvalue (.HitActor (Collision|BreakHitResult _array_element))))
      (if _returnvalue_3
        (Class|BPIDamagable|TakeDamage(Message) (.HitActor (Collision|BreakHitResult _array_element)) (stale Custom|Weapon%20Trace%20Start DamageInfo) _returnvalue)))))

(event Custom|Set%20Lock%20In%20Control%20Rotation
  ;[0.15 0.15 0.15 0.5] Lock In functionaliy
  (Pawn|SetControlRotation (Game|GetPlayerController 0) (Math|Rotator|FindLookatRotation (Transformation|GetActorLocation (Components|GetOwner)) (Transformation|GetActorLocation (Variables|Default|GetLockInActor)))))

(event Custom|Weapon%20Trace%20Start
  (params (BP%20weapon%20Base :type Actor%20Object%20Reference) (DamageInfo :type Damage%20Info%20Structure) (Radius :type Float%20%28single-precision%29))
  ;[0.15 0.15 0.15 0.5] Sword Trace Logic
  ;;[0.15 0.15 0.15 0.5] Sword Trece Timer Starts
  (bind _returnvalue (Utilities|Time|SetTimerbyEvent (EventDispatchers|CreateEvent :!event Custom|Trace) 0.0167 true))
  (Variables|Default|SetTraceTiemer _returnvalue)
  (bind _asbp_base_melee (Utilities|Casting|CastToBP_BaseMelee BP%20weapon%20Base)))

(event Custom|Weapon%20Trace%20End
  ;[0.15 0.15 0.15 0.5] Sword Trace Logic
  ;;[0.15 0.15 0.15 0.5] Sword Trace End
  (Utilities|Time|ClearandInvalidateTimerbyHandle (Variables|Default|GetTraceTiemer))
  (Utilities|Array|Clear (Variables|Default|GetActors%20to%20Ignore)))

(event EventTick
  (params (DeltaSeconds :type Float%20%28single-precision%29))
  ;[0.15 0.15 0.15 0.5] Lock In functionaliy
  ;;[0.15 0.126 0 0.5] Lock In Tick
  (if (Variables|Default|GetEnableTick)
    (Variables|Default|GetLockInActor
      (:then
        (CallFunction|SetLockinControlRotation))
      (:else))))

(event EventProjectileAttack
  (params (AttackInfo :type Projectile%20Info%20Structure%20%28by%20ref%29))
  (bind (_tracestart _traceend) (Utilities|Struct|BreakProjectileInfo AttackInfo))
  ;[0.15 0.07266 0.07266 0.84] Bullet Firing
  (Variables|Default|SetProjectile%20Info AttackInfo)
  (Utilities|Array|Clear (Variables|Default|GetActors%20to%20Ignore))
  (bind (_outhits _returnvalue) (Collision|MultiLineTraceByChannel _tracestart _traceend "TraceTypeQuery1" false (Variables|Default|GetActors%20to%20Ignore) "None"))
  (if _returnvalue
    (bind (_damagedactor _impact_location _enemyteam) (CallFunction|DamageFirstNonTeamMember _outhits (.DamageInfo (Utilities|Struct|BreakProjectileInfo (Variables|Default|GetProjectile%20Info)))))
    (Variables|Default|SetProjectile%20ImpactLocation _impact_location)
    (CallFunction|CheckifAllowedtoSpread)
    (bind _returnvalue_2 (Game|SpawnActorfromClass "/Game/Main/Wepon/Projectile/BP_ProjectileBase.BP_ProjectileBase_C" (Math|Transform|MakeTransform (.TraceStart (Utilities|Struct|BreakProjectileInfo (Variables|Default|GetProjectile%20Info))) (select (Variables|Default|GetSpread) (Math|Rotator|CombineRotators (Math|Rotator|FindLookatRotation (.TraceStart (Utilities|Struct|BreakProjectileInfo (Variables|Default|GetProjectile%20Info))) _impact_location) (Math|Rotator|MakeRotator 0.0 (Math|Random|RandomFloatinRange -1e+01 1e+01) (Math|Random|RandomFloatinRange -2.0 2.0))) (Math|Rotator|FindLookatRotation (.TraceStart (Utilities|Struct|BreakProjectileInfo (Variables|Default|GetProjectile%20Info))) _impact_location)) "1.000000,1.000000,1.000000") "Undefined" "MultiplyWithRoot" (Components|GetOwner) (.InitialSpeed (Utilities|Struct|BreakProjectileInfo (Variables|Default|GetProjectile%20Info))) (.Gravity (Utilities|Struct|BreakProjectileInfo (Variables|Default|GetProjectile%20Info))) 0))
    (bind _output_get (Variables|Default|SetProjectile%20Actor _returnvalue_2))
    (Collision|AssignOnComponentHit (Variables|/Game/Main/Wepon/Projectile/BP_ProjectileBase.BP_ProjectileBase_C|GetCollision%20Sphere _output_get) (EventDispatchers|CreateEvent :!event Custom|OnComponentHit_Event))
    (if _enemyteam
      (Collision|IgnoreActorwhenMoving (Variables|/Game/Main/Wepon/Projectile/BP_ProjectileBase.BP_ProjectileBase_C|GetCollision%20Sphere _output_get) (Components|GetOwner) true)
      (Class|BPIAI|TryAIMaleeBlock(Message) _damagedactor _output_get))))

(fn DamageFirstNonTeamMember
  (params (Hits :type Array%20of%20Hit%20Result%20Structures) (Damage%20Info :type Damage%20Info%20Structure))
  (bind _array_element (Utilities|Array|ForEachLoopwithBreak Hits :!label _label)
    (:LoopBody
      (bind _returnvalue (Class|GCharacterInterface|CheckifHostile(Message) (Components|GetOwner) (.HitActor (Collision|BreakHitResult _array_element))))
      (Utilities|FlowControl|Sequence
        (:then_0
          (goto _label Break))
        (:then_1
          (return (.HitActor (Collision|BreakHitResult _array_element)) (.ImpactPoint (Collision|BreakHitResult _array_element)) _returnvalue))))))

(fn AOEAttack
  (params (AOE%20info :type Struct%20AOE%20Structure) (Transform :type Transform))
  (bind (_aoeclass _damageinfo _radius _bdrawdebugsphere _ignoreinstigator _triggeronbeginplay) (Utilities|Struct|BreakStruct_AOE AOE%20info))
  (Variables|Default|SetAOE%20Info AOE%20info)
  (bind _returnvalue (Game|SpawnActorfromClass "/Game/AOE/BP_AOE_Base.BP_AOE_Base_C" Transform "Undefined" "MultiplyWithRoot" (Components|GetOwner) _radius _bdrawdebugsphere _ignoreinstigator _triggeronbeginplay 0))
  (bind _output_get (Variables|Default|SetAOE%20Actor _returnvalue))
  (EventDispatchers|BindEventtoOnAOEOverlapActor _output_get (EventDispatchers|CreateEvent :!event Custom|AOE%20Overlap))
  (Default|Trigger (Variables|Default|GetAOE%20Actor)))

(fn SetLockinActor
  (bind _returnvalue (Components|GetOwner))
  (bind _returnvalue_2 (Transformation|GetActorLocation _returnvalue))
  (Variables|Default|GetLockInActor
    (:then
      (Variables|Default|SetLockInActor 0)
      (Default|CallOnControllerFree))
    (:else
      (bind (_outhit _returnvalue_3) (Collision|SphereTraceForObjects _returnvalue_2 (+ _returnvalue_2 (* (Math|Vector|GetForwardVector (Transformation|GetWorldRotation (Variables|Default|GetFollowCamera))) 9e+04)) (Variables|Default|GetLockInTraceRadius) (Utilities|Array|MakeArray "ObjectTypeQuery3") false 0 "None"))
      (if _returnvalue_3
        (Variables|Default|SetLockInActor (.HitActor (Collision|BreakHitResult _outhit)))
        (Default|CallOnLockinActor)))))

(fn CheckifAllowedtoSpread
  (Variables|Default|SetAutoFiringCounter (+ (Variables|Default|GetAutoFiringCounter) 1))
  (if (>= (Variables|Default|GetAutoFiringCounter) (Variables|Default|GetHighestNonSpreadBulletCount))
    (Variables|Default|SetSpread true)
    (else
      (Variables|Default|SetSpread false))))